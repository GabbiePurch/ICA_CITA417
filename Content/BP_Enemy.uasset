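; BP_Enemy is a sphere enemy Blueprint that exercises a Health component with debug output.
; On BeginPlay it applies damage to the component, then heals it, printing current health on screen after each change.
; It binds the component's OnDeath event to print a death message, while overlap, Tick and the construction script do nothing.
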(event `self.ReceiveBeginPlay`
  (`HealthComponent.ApplyDamage` (`self.Health`) 20.0)
  (`KismetSystemLibrary.PrintString` (`KismetStringLibrary.Concat_StrStr` "Sphere (Enemy) Health: " (`KismetStringLibrary.Conv_DoubleToString` (`HealthComponent.GetCurrentHealth` (`self.Health`)))) true true (struct :`R` 1.0 :`G` 0.006104 :`A` 1.0) 5.0)
  (`KismetSystemLibrary.PrintString` "Adding Health:" true true (struct :`R` 1.0 :`A` 1.0) 5.0)
  (`HealthComponent.Heal` (`self.Health`) 5.0)
  (`KismetSystemLibrary.PrintString` (`KismetStringLibrary.Concat_StrStr` "Sphere (Enemy) Health: " (`KismetStringLibrary.Conv_DoubleToString` (`HealthComponent.GetCurrentHealth` (`self.Health`)))) true true (struct :`R` 1.0 :`G` 0.006104 :`A` 1.0) 5.0))

(event `self.Health.OnDeath`
  (`KismetSystemLibrary.PrintString` "SPHERE HAS DIED"))

(fn `UserConstructionScript`)